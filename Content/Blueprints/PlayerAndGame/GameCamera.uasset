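; GameCamera is the player's camera rig in a tower-stacking game, carrying the block spawner and indicator.
; Input slides the spawner smoothly or on a grid and spawns random blocks, with optional timed drops.
; A looping timer line-traces across the play space for the tower top, setting camera height, score and height and notifying TowerGameController.
; Tick eases the camera upward and decays bloom, grain and FOV kicks from PostProcessSet back to defaults.
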(event EventTick
  (params (DeltaSeconds :type Float%20%28single-precision%29))
  (bind _returnvalue (* DeltaSeconds 1.0))
  (bind _defaultsceneroot (Variables|Default|GetDefaultSceneRoot))
  ;[1 1 1] Move Camera
  (Transformation|SetWorldLocation _defaultsceneroot (Math|Vector|MakeVector 0.0 0.0 (Math|Float|Lerp (.z (Transformation|GetWorldLocation _defaultsceneroot)) (Variables|Default|GetcamHeight) (* DeltaSeconds 1e+01))) false false)
  ;[1 1 1] Update Post Processing
  (bind _output_get (Variables|Default|Setbloom (Math|Float|Lerp (Variables|Default|Getbloom) (Variables|Default|GetdefBloom) (* DeltaSeconds 2.0))))
  (bind _output_get_2 (Variables|Default|Setstatic (Math|Float|Lerp (Variables|Default|Getstatic) (Variables|Default|GetdefStatic) _returnvalue)))
  (Variables|Default|Setfov (Math|Float|Lerp (Variables|Default|Getfov) (Variables|Default|GetdefFov) _returnvalue))
  (Variables|/Script/Engine.PostProcessComponent|SetSettings (Variables|Default|GetPostProcess) (Utilities|Struct|MakePostProcessSettings "AEM_Manual" _output_get 0.1 11.0 _output_get_2 (Variables|Default|GetPost%20Process%20Materials)))
  (Camera|SetFieldOfView (Variables|Default|GetCamera) (Variables|Default|Getfov)))

(event EventBeginPlay
  (bind _postprocess (Variables|Default|GetPostProcess))
  (bind _settings (Variables|/Script/Engine.PostProcessComponent|GetSettings _postprocess))
  (bind (_bloomintensity _grainintensity _weightedblendables) (Utilities|Struct|BreakPostProcessSettings _settings))
  (Utilities|Time|SetTimerbyFunctionName 0 "SetNewHeight" 0.1 true)
  (if (Variables|Default|GetisTimerUsed)
    (Utilities|Time|SetTimerbyFunctionName 0 "FallingObjectLoop" (Variables|Default|GettimerWait) true)
    (else
      (CallFunction|LoadNextObject)))
  (bind _output_get (Variables|Default|SetdefBloom _bloomintensity))
  (Variables|Default|Setbloom _output_get)
  (bind _output_get_2 (Variables|Default|SetdefStatic _grainintensity))
  (Variables|Default|Setstatic _output_get_2)
  (bind _output_get_3 (Variables|Default|SetdefFov (Variables|/Script/Engine.CameraComponent|GetFieldOfView (Variables|Default|GetCamera))))
  (Variables|Default|Setfov _output_get_3)
  (Variables|Default|SetPost%20Process%20Materials _weightedblendables))

(event Input|ActionEvents|InputActionPlace
  (params (Key :type Key%20Structure :default "None"))
  (bind _indicatormesh (Variables|Default|GetindicatorMesh))
  ;[0.633 1 0.6611] SPAWNING BLOCKS
  (:Pressed
    (Utilities|FlowControl|DoOnce false :!label _label
      (:Completed
        (if (Variables|Default|GetisTimerUsed)
          (Utilities|Time|SetTimerbyFunctionName 0 "FallingObjectLoop" (Variables|Default|GettimerWait) true)
          (else
            (CallFunction|FallingObjectLoop)))
        (Rendering|Material|SetMaterial _indicatormesh 0 "/Game/Art/Materials/outlineFade.outlineFade")
        (Utilities|FlowControl|Delay 1.0)
        (Rendering|Material|SetMaterial _indicatormesh 0 "/Game/Art/Materials/basicWhite.basicWhite")
        (goto _label Reset)))))

(event Input|ActionEvents|InputActionSnapMoveBlockLeft
  (params (Key :type Key%20Structure :default "None"))
  (bind _physicsobjectspawner (Variables|Default|GetPhysicsObjectSpawner))
  (bind _relativelocation (Variables|/Script/Engine.SceneComponent|GetRelativeLocation _physicsobjectspawner))
  ;[0.5979 0.7549 1] MOVE SPAWNER GRID
  (:Pressed
    (Utilities|FlowControl|DoOnce false :!label _label
      (:Completed
        (Transformation|SetRelativeLocation (Variables|Default|GetPhysicsObjectSpawner) (Math|Vector|MakeVector (.x _relativelocation) (- (.y _relativelocation) 1e+02) (.z _relativelocation)) false false))))
  (:Released
    (goto _label Reset)))

(event Input|ActionEvents|InputActionSnapMoveBlockRight
  (params (Key :type Key%20Structure :default "None"))
  (bind _physicsobjectspawner (Variables|Default|GetPhysicsObjectSpawner))
  (bind _relativelocation (Variables|/Script/Engine.SceneComponent|GetRelativeLocation _physicsobjectspawner))
  ;[0.5979 0.7549 1] MOVE SPAWNER GRID
  (:Pressed
    (Utilities|FlowControl|DoOnce false :!label _label
      (:Completed
        (Transformation|SetRelativeLocation (Variables|Default|GetPhysicsObjectSpawner) (Math|Vector|MakeVector (.x _relativelocation) (+ (.y _relativelocation) 1e+02) (.z _relativelocation)) false false))))
  (:Released
    (goto _label Reset)))

(event Input|ActionEvents|InputActionSnapToGrid
  (params (Key :type Key%20Structure :default "None"))
  (bind _physicsobjectspawner (Variables|Default|GetPhysicsObjectSpawner))
  (bind _relativelocation (Variables|/Script/Engine.SceneComponent|GetRelativeLocation _physicsobjectspawner))
  ;[0.5979 0.7549 1] MOVE SPAWNER GRID
  (:Pressed
    (Utilities|FlowControl|DoOnce false :!label _label
      (:Completed
        (Transformation|SetRelativeLocation _physicsobjectspawner (Math|Vector|MakeVector (.x _relativelocation) (Math|Float|SnapToGrid(Float) (.y _relativelocation) 1e+02) (.z _relativelocation)) false false))))
  (:Released
    (goto _label Reset)))

(event Input|AxisEvents|InputAxisSmoothMoveBlock
  (params (AxisValue :type Float%20%28single-precision%29))
  (bind _returnvalue (Utilities|Time|GetWorldDeltaSeconds))
  (bind _physicsobjectspawner (Variables|Default|GetPhysicsObjectSpawner))
  (bind _relativelocation (Variables|/Script/Engine.SceneComponent|GetRelativeLocation _physicsobjectspawner))
  ;[1 0.3594 0.3594] MOVE SPAWNER SMOOTH
  (if (== AxisValue 0.0)
    ;;[1 1 1] Decrease Acceleration
    (Variables|Default|Setacceleration (Math|Float|Lerp (Variables|Default|Getacceleration) 0.0 (* _returnvalue 1e+01)))
    (else
      ;;[1 1 1] Increase Acceleration
      (bind _output_get (Variables|Default|Setacceleration (Math|Float|Clamp(Float) (+ (* AxisValue _returnvalue 3e+01) (Variables|Default|Getacceleration)) -1e+01 1e+01)))))
  ;;[1 1 1] Add The Acceleration
  (Transformation|AddLocalOffset (Variables|Default|GetPhysicsObjectSpawner) (* "0,1.000000, 0" _output_get) false false)
  ;;[1 1 1] Clamp Blocks Within Playspace
  (if (or (> (.y _relativelocation) 1e+03) (< (.y _relativelocation) -1e+03))
    (Transformation|SetRelativeLocation _physicsobjectspawner (Math|Vector|MakeVector (.x _relativelocation) (Math|Float|Clamp(Float) (.y _relativelocation) -1e+03 1e+03) (.z _relativelocation)) false false)
    (Variables|Default|Setacceleration 0.0)))

(fn ConstructionScript)

(fn SpawnObject
  (Game|SpawnActorfromClass (Variables|Default|GetnextPhysicsObject) (Transformation|GetWorldTransform (Variables|Default|GetPhysicsObjectSpawner)) "Undefined" 0 0))

(fn LoadNextObject
  (bind _blockrow (Variables|Default|GetblockRow))
  ;[1 1 1] Select next item to be spawned
  (LocalVariables|SetselectedIndex (Math|Random|RandomInteger (Utilities|Array|Length _blockrow)))
  ;[1 1 1] Set next physical object and outline
  (Variables|Default|SetnextPhysicsObject (.physicsObject (Utilities|Struct|BreakBlocksRow (Utilities|Array|Get(acopy) _blockrow (LocalVariables|GetselectedIndex)))))
  (Components|StaticMesh|SetStaticMesh (Variables|Default|GetindicatorMesh) (.outlineObject (Utilities|Struct|BreakBlocksRow (Utilities|Array|Get(acopy) _blockrow (LocalVariables|GetselectedIndex))))))

(fn FallingObjectLoop
  (CallFunction|SpawnObject)
  (CallFunction|LoadNextObject))

(fn SetNewHeight
  ;[1 1 1] Check If Game Has Ended, Or In Practice
  (if (Variables|Default|GetisPractice)
    (for _index (range 0 21) :!label _label
      ;[1 1 1] Check Along Play Space For Tallest Height
      (bind _outhit (Collision|LineTraceByChannel (+ (Transformation|GetWorldLocation (Variables|Default|GetRaycastChecker)) (Math|Vector|MakeVector 0.0 (* _index 97.0) 0.0)) (- (+ (Transformation|GetWorldLocation (Variables|Default|GetRaycastChecker)) (Math|Vector|MakeVector 0.0 (* _index 97.0) 0.0)) (Math|Vector|MakeVector 0.0 0.0 1.5e+04)) "TraceTypeQuery3" false 0 "None" true "(R=1.000000,G=0.000000,B=0.000000,A=1.000000)" "(R=0.000000,G=1.000000,B=0.000000,A=1.000000)" 1.0))
      (if (.bBlockingHit (Collision|BreakHitResult _outhit))
        (if (Utilities|Enum|Equal(Enum) (Collision|GetCollisionObjectType (.HitComponent (Collision|BreakHitResult _outhit))) "ECC_GameTraceChannel1")
          (if (< (LocalVariables|GetcurrentNewHeight) (.z (.Location (Collision|BreakHitResult _outhit))))
            (LocalVariables|SetcurrentNewHeight (.z (.Location (Collision|BreakHitResult _outhit))))))))
    ;[1 1 1] Set Camera Height
    (Variables|Default|SetcamHeight (Math|Float|SnapToGrid(Float) (Math|Float|Clamp(Float) (LocalVariables|GetcurrentNewHeight) 0.0 1e+06) 1e+01))
    (Variables|Default|Setscore (Math|Float|Truncate (Math|Float|SnapToGrid(Float) (Math|Float|Clamp(Float) (+ (LocalVariables|GetcurrentNewHeight) 7.5e+02) 0.0 1e+06) 1.0)))
    (Variables|Default|Setheight (/ (Math|Float|SnapToGrid(Float) (Math|Float|Clamp(Float) (+ (LocalVariables|GetcurrentNewHeight) 7.5e+02) 0.0 1e+06) 1.0) 1e+02))
    (bind _astower_game_controller (Utilities|Casting|CastToTowerGameController (Game|GetPlayerController 0)))
    (Default|UpdateGameVariables _astower_game_controller)
    (else
      (bind _astower_game_controller_2 (Utilities|Casting|CastToTowerGameController (Game|GetPlayerController 0)))
      (if (not (Variables|/Game/Blueprints/PlayerAndGame/TowerGameController.TowerGameController_C|GetgameEnded _astower_game_controller_2))
        (goto _label)))))

(fn PostProcessSet
  (params (addBloom :type Float%20%28single-precision%29) (addStatic :type Float%20%28single-precision%29) (addFov :type Float%20%28single-precision%29))
  (Variables|Default|Setbloom (Math|Float|Clamp(Float) (+ (Variables|Default|Getbloom) addBloom) 0.0 7.0))
  (Variables|Default|Setstatic (Math|Float|Clamp(Float) (+ addStatic (Variables|Default|Getstatic)) 0.0 0.6))
  (Variables|Default|Setfov (Math|Float|Clamp(Float) (+ addFov (Variables|Default|Getfov)) 0.0 75.0)))