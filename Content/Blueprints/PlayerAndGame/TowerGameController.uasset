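; Player controller for the tower game that manages the HUD, music, pause menu and end of round.
; On BeginPlay it reads IsPractice from the GameCamera pawn to choose the music and whether to start a 60-second timer that calls EndGame.
; UpdateGameVariables pushes the pawn's score and height, plus remaining time, to the HUD.
; Pausing binds PauseMenu buttons to resume or title exit; EndGame disables input and shows ScoreMenu.
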(event Custom|UpdateGameVariables
  ;[1 1 1] Update Game Variables and HUD
  (bind _asgame_camera (Utilities|Casting|CastToGameCamera (Game|Player|GetPlayerPawn 0)))
  (bind _output_get (Variables|Default|Setscore (Variables|/Game/Blueprints/PlayerAndGame/GameCamera.GameCamera_C|Getscore _asgame_camera)))
  (bind _output_get_2 (Variables|Default|Setheight (Variables|/Game/Blueprints/PlayerAndGame/GameCamera.GameCamera_C|Getheight _asgame_camera)))
  (Default|UpdateHUD (Variables|Default|GetHUD) _output_get _output_get_2 (Utilities|Time|GetTimerRemainingTimebyHandle (Variables|Default|Gettimer))))

(event Custom|Unpause%20Game
  (bind _self self)
  (if (not (Variables|Default|GetgameEnded))
    (Game|SetGamePaused false)
    (Class|AudioComponent|SetPaused (Variables|Default|Getmusic) false)
    ;[1 1 1] Input to Game
    (Input|SetInputModeGameOnly _self)
    (Variables|Default|SetbShowMouseCursor _self false)
    ;[1 1 1] Remove Pause Widget
    (Widget|SetRenderOpacity (Variables|Default|GetHUD) 1.0)
    (Utilities|IsValid (Variables|Default|GetpauseMenu)
      (:Is%20Valid
        (EventDispatchers|UnbindallEventsfromResumeBttnClicked (Variables|Default|GetpauseMenu))
        (EventDispatchers|UnbindallEventsfromExitBttnClicked (Variables|Default|GetpauseMenu))
        (Widget|RemovefromParent (Variables|Default|GetpauseMenu))
        (Variables|Default|SetpauseMenu 0)))))

(event Custom|Pause%20Game
  (bind _self self)
  (if (not (Variables|Default|GetgameEnded))
    (Game|SetGamePaused true)
    (Class|AudioComponent|SetPaused (Variables|Default|Getmusic) true)
    ;[1 1 1] Input to Game/UI
    (Input|SetInputModeGameandUI _self 0 "DoNotLock" false)
    (Variables|Default|SetbShowMouseCursor _self true)
    ;[1 1 1] Add Pause Widget
    (Widget|SetRenderOpacity (Variables|Default|GetHUD) 0.0)
    (bind _returnvalue (UserInterface|CreateWidget "/Game/Blueprints/GUI/PauseMenu.PauseMenu_C"))
    (bind _output_get (Variables|Default|SetpauseMenu _returnvalue))
    (UserInterface|Viewport|AddtoPlayerScreen _output_get)
    (EventDispatchers|BindEventtoResumeBttnClicked _output_get (delegate Custom|Unpause%20Game))
    (EventDispatchers|BindEventtoExitBttnClicked _output_get (delegate Custom|ExitTitle))))

(event Custom|ExitTitle
  (CallFunction|UnpauseGame)
  (Game|OpenLevel(byName) "TitleScreen"))

(event EventBeginPlay
  (bind _self self)
  ;[1 1 1] BeginPlay
  (Input|SetInputModeGameOnly _self)
  (Variables|Default|SetbShowMouseCursor _self false)
  (bind _asgame_camera (Utilities|Casting|CastToGameCamera (Game|Player|GetPlayerPawn 0)))
  (Variables|Default|SetisPractice (Variables|/Game/Blueprints/PlayerAndGame/GameCamera.GameCamera_C|GetisPractice _asgame_camera))
  (bind _returnvalue (UserInterface|CreateWidget "/Game/Blueprints/GUI/TowerHUD_Basic.TowerHUD_Basic_C"))
  (bind _output_get (Variables|Default|SetHUD _returnvalue))
  (UserInterface|Viewport|AddtoViewport _output_get 0)
  (bind _returnvalue_2 (UserInterface|CreateWidget "/Game/Blueprints/GUI/TowerHUD_ScreenOverlay.TowerHUD_ScreenOverlay_C"))
  (UserInterface|Viewport|AddtoViewport _returnvalue_2 0)
  (if (Variables|Default|GetisPractice)
    (bind _returnvalue_3 (Audio|SpawnSound2D "/Game/Art/Audio/Walking.Walking" 1.0 1.0 0.0 0))
    (Variables|Default|Setmusic _returnvalue_3)
    (else
      (bind _returnvalue_4 (Utilities|Time|SetTimerbyFunctionName self "EndGame" 6e+01))
      (Variables|Default|Settimer _returnvalue_4)
      (bind _returnvalue_5 (Audio|SpawnSound2D "/Game/Art/Audio/Score.Score" 1.0 1.0 0.0 0))
      (Variables|Default|Setmusic _returnvalue_5))))

(event Input|ActionEvents|InputActionPause
  (params (Key :type Key%20Structure :default "None"))
  ;[1 1 1] Toggle Game Pause
  (:Pressed
    (if (Game|IsGamePaused)
      (Default|PauseUndone (Variables|Default|GetpauseMenu))
      (else
        (CallFunction|PauseGame)))))

(fn ConstructionScript)

(fn EndGame
  (bind _self self)
  ;[1 1 1] Disable Player
  (Variables|Default|SetgameEnded true)
  (Input|DisableInput (Game|Player|GetPlayerPawn 0) (Game|GetPlayerController 0))
  ;[1 1 1] Disable Gameplay HUD
  (Variables|Default|SetpauseMenu 0)
  (Widget|SetRenderOpacity (Variables|Default|GetHUD) 0.0)
  (Variables|Default|SetHUD 0)
  ;[1 1 1] Spawn Endgame HUD
  (bind _returnvalue (UserInterface|CreateWidget "/Game/Blueprints/GUI/ScoreMenu.ScoreMenu_C"))
  (UserInterface|Viewport|AddtoPlayerScreen _returnvalue)
  ;[1 1 1] Input to Game/UI
  (Input|SetInputModeUIOnly _self _returnvalue "DoNotLock")
  (Variables|Default|SetbShowMouseCursor _self true))