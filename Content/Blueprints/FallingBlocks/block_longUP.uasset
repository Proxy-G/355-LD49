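; Falling block Blueprint (long upright variant, by its name) that reacts to the first physical impact of its static mesh.
; A one-shot flag gates the hit event, which then switches the mesh's collision object type and channel response so camera raycasts detect it.
; The same hit spawns an impact particle, plays a pitch-randomized placement sound and triggers a bloom, static and FOV post-process effect on the GameCamera pawn.
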(event OnComponentHit(StaticMesh)
  (params (HitComponent :type Primitive%20Component%20Object%20Reference) (OtherActor :type Actor%20Object%20Reference) (OtherComp :type Primitive%20Component%20Object%20Reference) (NormalImpulse :type Vector :default "0, 0, 0") (Hit :type Hit%20Result%20Structure%20%28by%20ref%29))
  ;[1 1 1] Make Sure First Hit
  (if (not (Variables|Default|GetinitialHit))
    (Variables|Default|SetinitialHit true)
    ;[1 1 1] Set Collision To Be Seen By  Cam Raycasts
    (Collision|SetCollisionObjectType (Variables|Default|GetStaticMesh) "ECC_GameTraceChannel1")
    (Collision|SetCollisionResponsetoChannel (Variables|Default|GetStaticMesh) "ECC_GameTraceChannel2" "ECR_Block")
    ;[1 1 1] Spawn Particles + Play Sound
    (Effects|SpawnEmitteratLocation "/Game/Art/ParticleEffects/PhysicsBlockInitialCollision.PhysicsBlockInitialCollision" (Transformation|GetWorldLocation (Variables|Default|GetStaticMesh)) "0, 0, 0" "1.000000,1.000000,1.000000" true "AutoRelease")
    (Audio|PlaySound2D "/Game/Art/Audio/sfx_blockPlace.sfx_blockPlace" 1.0 (Math|Random|RandomFloatinRange 0.85 1.15) 0.0 0 0)
    ;[1 1 1] Do Post Process Effects
    (bind _asgame_camera (Utilities|Casting|CastToGameCamera (Game|Player|GetPlayerPawn 0)))
    (Default|PostProcessSet _asgame_camera 3.0 0.2 1.0)))

(fn ConstructionScript)